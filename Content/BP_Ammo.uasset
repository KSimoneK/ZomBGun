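; BP_Ammo is an ammo pickup that destroys itself when any actor overlaps it.
; Tick casts the player to BP_ThirdPersonCharacter and copies its Ammo into a local variable.
; Overlap adds a fixed amount to that copy with a cap, prints it and re-adds existing WB_Ammo widgets to the viewport, without writing back to the character.
; An AddAmmo function repeats the capped addition but is not called here.
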(event `self.ReceiveBeginPlay`)

(event `self.ReceiveTick`
  (params (DeltaSeconds :type "Float (single-precision)"))
  (bind _asbp_third_person_character (cast `/Game/ThirdPerson/Blueprints/BP_ThirdPersonCharacter` (`GameplayStatics.GetPlayerCharacter` 0)))
  (bind _output_get (set `self.As BP Third Person Character` _asbp_third_person_character))
  (bind _output_get_2 (set `self.Ammo` (`/Game/ThirdPerson/Blueprints/BP_ThirdPersonCharacter.Ammo` _output_get))))

(event `self.ReceiveActorBeginOverlap`
  (params (OtherActor :type "Actor Object Reference"))
  (bind _ammo (`self.Ammo`))
  (`self.K2_DestroyActor`)
  (set `self.Ammo` (+ (`self.Ammo`) 16))
  (if (> (`self.Ammo`) 48)
    (set `self.Ammo` (- _ammo (- _ammo 48))))
  (`KismetSystemLibrary.PrintString` (`KismetStringLibrary.Conv_IntToString` (stale `self.ReceiveTick` _output_get_2)))
  (bind _foundwidgets (`WidgetBlueprintLibrary.GetAllWidgetsOfClass` "/Game/WB_Ammo.WB_Ammo_C" false))
  (`UserWidget.AddToViewport` _foundwidgets 0))

(fn `AddAmmo`
  (bind _ammo (`self.Ammo`))
  (bind _ammo_2 (`self.Ammo`))
  (set `self.Ammo` (+ (`self.Ammo`) 16))
  (if (> _ammo_2 48)
    (set `self.Ammo` (- _ammo (- _ammo 48)))
    (`KismetSystemLibrary.PrintString` (`KismetStringLibrary.Conv_IntToString` _ammo_2))))

(fn `UserConstructionScript`)