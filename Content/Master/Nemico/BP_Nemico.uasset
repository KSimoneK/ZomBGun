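; Enemy character that roams randomly, chases the player when spotted and attacks in melee.
; Roaming loops through AI MoveTo to random reachable points; PawnSensing switches to a faster chase, and a retriggerable delay returns it to slower roaming once sight is lost.
; Attacks play a montage whose notify triggers a sphere-overlap damage check.
; Damage lowers clamped Health, and Tick triggers a random death animation before destroying the actor.
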(event `RoamNemico`
  ; Roam Del Nemico
  (`|AIMoveTo` self (`NavigationSystemV1.K2_GetRandomReachablePointInRadius` (`self.K2_GetActorLocation`) 1500.0 null null) null
    (:`OnSuccess`
      (`KismetSystemLibrary.Delay` 2.0)
      (`self.RoamNemico`))))

(event `self.ReceiveBeginPlay`
  ; Roam Del Nemico
  (`self.RoamNemico`))

(event `self.PawnSensing.OnSeePawn`
  (params (Pawn :type "Pawn Object Reference"))
  ; Inseguimento Mostro
  (set `self.CanAttack` true)
  (`|ExecutionSequence`
    (:`then_0`
      (set `CharacterMovementComponent.MaxWalkSpeed` 200.0 (`self.CharacterMovement`))
      (`|AIMoveTo` self (0.0 0.0 0.0) (`GameplayStatics.GetPlayerCharacter` 0) 70.0
        (:`OnSuccess`
          (if (`self.CanAttack`)
            (`self.Attack`)
            (set `self.CanAttack` false)))))
    (:`then_1`
      (`KismetSystemLibrary.RetriggerableDelay` 1.0)
      (`self.RoamNemico`)
      (set `CharacterMovementComponent.MaxWalkSpeed` 100.0 (`self.CharacterMovement`)))))

(event `Attack`
  ; Attacco Nemico
  (`/Engine/EditorBlueprintResources/StandardMacros.DoOnce` false :!label _label
    (:`Completed`
      (`CharacterMovementComponent.DisableMovement` (`self.CharacterMovement`))
      (`|PlayMontage` (`self.Mesh`) "/Game/Master/Nemico/AM_Nemico.AM_Nemico"
        (:`OnCompleted`
          (`KismetSystemLibrary.Delay` 0.4)
          (set `self.CanAttack` true)
          (`CharacterMovementComponent.SetMovementMode` (`self.CharacterMovement`) "MOVE_Walking" 0)
          (goto _label :!via `Reset`))
        (:`OnNotifyBegin`
          (`self.DealDamage`))))))

(event `self.ReceiveTick`
  (params (DeltaSeconds :type "Float (single-precision)"))
  ; Death
  (if (<= (`self.Health`) 0.0)
    (`/Engine/EditorBlueprintResources/StandardMacros.DoOnce` false
      (:`Completed`
        (`self.Death`)))))

(event `self.ReceiveAnyDamage`
  (params (Damage :type "Float (single-precision)") (DamageType :type "DamageType Object Reference") (InstigatedBy :type "Controller Object Reference") (DamageCauser :type "Actor Object Reference"))
  ; Is Damaged
  (set `self.Health` (`KismetMathLibrary.FClamp` (- (`self.Health`) Damage) 0.0 (`self.MaxHealth`))))

(event `Death`
  ; Death
  (`CharacterMovementComponent.DisableMovement` (`self.CharacterMovement`))
  (`SkeletalMeshComponent.PlayAnimation` (`self.Mesh`) (`KismetArrayLibrary.Array_Random` (`self.DeathAnim`)) false)
  (`PrimitiveComponent.SetCollisionEnabled` (`self.CapsuleComponent`) "NoCollision")
  (`KismetSystemLibrary.Delay` 5.0)
  (`self.K2_DestroyActor`))

(event `DealDamage`
  ; Deal Damage
  (bind _outactors (`KismetSystemLibrary.SphereOverlapActors` (`SceneComponent.K2_GetComponentLocation` (`self.AttackSphere`)) 32.0 (`|MakeArray` "ObjectTypeQuery3" :!type "EObjectTypeQuery Enum") "/Script/Engine.Actor" (`|MakeArray` self :!type "Actor Object Reference")))
  (for _array_element _outactors
    (`GameplayStatics.ApplyDamage` _array_element (`self.Base Damage`) (`self.GetController`) self "/Script/Engine.DamageType")))

(fn `UserConstructionScript`)